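; BP_ERPlayerController is a player controller that seeds the player's starting inventory and provides hotkeys that appear to test equipping.
; On BeginPlay it adds Artorias armor pieces, a spear and arrows from DataTables through InventoryAC, then equips each returned item.
; Keys 4, 5 and 6 respectively add a Partizan, equip that stored item to the RHand3 slot and clear that slot.
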(event `Key|Six`
  (params (Key :type "Key Structure"))
  (:`Pressed`
    (`InventoryAC.ClearEquipSlot` (`self.InventoryAC`) "RHand3")))

(event `Key|Five`
  (params (Key :type "Key Structure"))
  (:`Pressed`
    (`InventoryAC.SetEquipItemToSlot` (`self.InventoryAC`) (stale `Key|Four` _returnvalue) "RHand3")))

(event `Key|Four`
  (params (Key :type "Key Structure"))
  (:`Pressed`
    (bind _returnvalue (`InventoryAC.AddItem` (`self.InventoryAC`) (make `DataTableRowHandle` "/Game/Inventory/Data/DT_Weapons.DT_Weapons" "Partizan") 1))))

(event `self.ReceiveBeginPlay`
  (bind _inventoryac (`self.InventoryAC`))
  (bind _returnvalue (`InventoryAC.SetItems` _inventoryac (`|MakeArray` (make `InventorySlot` (make `DataTableRowHandle` "/Game/Inventory/Data/DT_Armors.DT_Armors" "ArtoriasArmor") 2) (make `InventorySlot` (make `DataTableRowHandle` "/Game/Inventory/Data/DT_Boots.DT_Boots" "ArtoriasBoots")) (make `InventorySlot` (make `DataTableRowHandle` "/Game/Inventory/Data/DT_Gloves.DT_Gloves" "ArtoriasGloves")) (make `InventorySlot` (make `DataTableRowHandle` "/Game/Inventory/Data/DT_Helms.DT_Helms" "ArtoriasHelm")) (make `InventorySlot` (make `DataTableRowHandle` "/Game/Inventory/Data/DT_Weapons.DT_Weapons" "Spear")) (make `InventorySlot` (make `DataTableRowHandle` "/Game/Inventory/Data/DT_Arrows.DT_Arrows" "Arrow") 6) :!type "InventorySlot Structure") false))
  (for _array_element _returnvalue
    (`InventoryAC.SetEquipItem` _inventoryac _array_element)))

(fn `UserConstructionScript`)